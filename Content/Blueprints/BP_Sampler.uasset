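; BP_Sampler voxelizes a target actor by sampling orthographic depth captures from a list of directions.
; For each direction, it frames the target's voxel-snapped bounds with a show-only scene capture, using one pixel per voxel.
; It converts depth pixels below a far cutoff into grid-aligned world positions, capturing only visible surfaces.
; Each pass spawns an instanced-mesh actor from those voxels, though Transforms is never cleared between passes.
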(event EventBeginPlay)

(event Collision|EventActorBeginOverlap
  (params (OtherActor :type Actor%20Object%20Reference)))

(event EventTick
  (params (DeltaSeconds :type Float%20%28single-precision%29)))

(fn ConstructionScript)

(fn ShowBound
  (bind _sampletarget (Variables|Default|GetSampleTarget))
  (bind (_origin _boxextent) (Collision|GetActorBounds _sampletarget false false))
  (Rendering|Debug|DrawDebugBox _origin (CallFunction|SnapExtenttoVoxelSize _boxextent) "(R=1.000000,G=0.914658,B=0.225686,A=1.000000)" "0, 0, 0" 1e+01 2.0))

(fn 1SetView
  (bind _scenecapturecomponent2d (Variables|Default|GetSceneCaptureComponent2D))
  (bind _sampletarget (Variables|Default|GetSampleTarget))
  (bind _sampledirection (Variables|Default|GetSampleDirection))
  (bind _voxelsize (Variables|Default|GetVoxelSize))
  (bind (_origin _boxextent) (Collision|GetActorBounds _sampletarget false false))
  (bind _returnvalue (CallFunction|SnapExtenttoVoxelSize _boxextent))
  (bind _returnvalue_2 (+ _origin ""))
  (bind _returnvalue_3 (* _returnvalue "2.000000,2.000000,2.000000"))
  (bind _returnvalue_4 (* _returnvalue _sampledirection))
  (bind _returnvalue_5 (- _returnvalue_2 _returnvalue_4))
  (bind _returnvalue_6 (Math|Rotator|FindLookatRotation _returnvalue_5 _origin))
  (bind _returnvalue_7 (Math|Vector|RotateVector _returnvalue_3 _returnvalue_6))
  (bind _returnvalue_8 (Math|Vector|VectorGetAbs _returnvalue_7))
  (bind (_x _y _z) (Math|Vector|BreakVector _returnvalue_8))
  (bind _returnvalue_9 (Math|Float|Round _x))
  (bind _returnvalue_10 (Math|Float|Round _y))
  (bind _returnvalue_11 (Math|Float|Round _z))
  (bind _returnvalue_12 (Math|Conversions|ToFloat(Integer) _returnvalue_9))
  (bind _returnvalue_13 (Math|Conversions|ToFloat(Integer) _returnvalue_10))
  (bind _returnvalue_14 (Math|Conversions|ToFloat(Integer) _returnvalue_11))
  (bind _returnvalue_15 (Math|Vector|MakeVector _returnvalue_12 _returnvalue_13 _returnvalue_14))
  (bind _returnvalue_16 (/ _returnvalue_15 _voxelsize))
  (bind (_x_2 _y_2 _z_2) (Math|Vector|BreakVector _returnvalue_16))
  (Transformation|SetWorldLocationAndRotation (Variables|Default|GetSceneCaptureComponent2D) _returnvalue_5 _returnvalue_6 false false)
  (Variables|/Script/Engine.SceneCaptureComponent2D|SetOrthoWidth (Variables|Default|GetSceneCaptureComponent2D) (.Y (Math|Vector|BreakVector _returnvalue_15)))
  (bind _returnvalue_17 (Rendering|CreateRenderTarget2D (Math|Float|Ceil _y_2) (Math|Float|Ceil _z_2) "RTF_RGBA16f"))
  (bind _output_get (Variables|Default|SetRT_Depth _returnvalue_17))
  (bind _output_get_2 (Variables|/Script/Engine.SceneCaptureComponent2D|SetTextureTarget (Variables|Default|GetSceneCaptureComponent2D) _output_get))
  (bind _returnvalue_18 (Rendering|Material|CreateDynamicMaterialInstance (Variables|Default|GetPreview) 0 "/Game/Material/Preview_Instance.Preview_Instance" "None" :!class /Script/Engine.PrimitiveComponent))
  (Rendering|Material|SetTextureParameterValue _returnvalue_18 "Preview Texture" _output_get_2)
  (Rendering|SceneCapture|ClearShowOnlyComponents _scenecapturecomponent2d)
  (Rendering|SceneCapture|ShowOnlyActorComponents _scenecapturecomponent2d (Variables|Default|GetSampleTarget) false)
  (Rendering|SceneCapture|CaptureScene _scenecapturecomponent2d :!class /Script/Engine.SceneCaptureComponent2D))

(fn 2Sample
  (bind _rt_depth (Variables|Default|GetRT_Depth))
  (bind _sizex (Variables|/Script/Engine.TextureRenderTarget2D|GetSizeX _rt_depth))
  (Utilities|Array|Clear (Variables|Default|GetVoxels))
  (bind _outlinearsamples (Class|KismetRenderingLibrary|ReadRenderTargetRaw (Variables|Default|GetRT_Depth) false))
  (for (_array_element _array_index) _outlinearsamples
    (if (< (.R (Utilities|Struct|BreakLinearColor _array_element)) 6.55e+05)
      (Utilities|Array|Add (Variables|Default|GetVoxels) (Utilities|Struct|MakeVoxel (CallFunction|RTSpacetoWorldSpace (.R (Utilities|Struct|BreakLinearColor _array_element)) (Math|Conversions|ToFloat(Integer) (Math|Integer|%(Integer) _array_index _sizex)) (Math|Conversions|ToFloat(Integer) (- (- (Variables|/Script/Engine.TextureRenderTarget2D|GetSizeY _rt_depth) (/ _array_index _sizex)) 1)) (Transformation|GetWorldTransform (Variables|Default|GetSceneCaptureComponent2D)) (Variables|Default|GetRT_Depth)))))))

(fn 3BuildInstanceMesh
  (bind _sampletarget (Variables|Default|GetSampleTarget))
  (bind _transforms (LocalVariables|GetTransforms))
  (bind _returnvalue (Transformation|GetActorLocation _sampletarget))
  (bind _returnvalue_2 (Game|SpawnActorfromClass "/Game/Blueprints/Voxelization/InstanceStaticMeshActor.InstanceStaticMeshActor_C" (Math|Conversions|ToTransform(Vector) _returnvalue) "Undefined" "MultiplyWithRoot" 0 0))
  (for _array_element (Variables|Default|GetVoxels)
    (Utilities|Array|Add _transforms (Math|Transform|MakeTransform (- (Utilities|Struct|BreakVoxel _array_element) _returnvalue) "0, 0, 0" (Math|Conversions|ToVector(Float) (Variables|Default|GetVoxelSize)))))
  (Components|InstancedStaticMesh|AddInstances (Variables|/Game/Blueprints/Voxelization/InstanceStaticMeshActor.InstanceStaticMeshActor_C|GetInstancedStaticMesh _returnvalue_2) _transforms false false true)
  (return))

(fn RTSpacetoWorldSpace
  (params (Depth :type Float%20%28double-precision%29) (X :type Float%20%28double-precision%29) (Y :type Float%20%28double-precision%29) (View%20Transform :type Transform) (RT :type Texture%20Render%20Target%202D%20Object%20Reference))
  (bind (_location _rotation) (Math|Transform|BreakTransform View%20Transform))
  (return (Math|Transform|TransformLocation (Math|Transform|MakeTransform _location _rotation (Math|Conversions|ToVector(Float) (Variables|Default|GetVoxelSize))) (+ (Math|Vector|MakeVector (Math|Conversions|ToFloat(Integer) (Math|Float|Floor (/ Depth (Variables|Default|GetVoxelSize)))) (- X (/ (Math|Conversions|ToFloat(Integer) (Variables|/Script/Engine.TextureRenderTarget2D|GetSizeX RT)) 2.0)) (- Y (/ (Math|Conversions|ToFloat(Integer) (Variables|/Script/Engine.TextureRenderTarget2D|GetSizeY RT)) 2.0))) "0.500000,0.500000,0.500000"))))

(fn SnapExtenttoVoxelSize
  (params (Extent :type Vector))
  (bind _voxelsize (Variables|Default|GetVoxelSize))
  (bind _returnvalue (/ Extent _voxelsize))
  (bind (_x _y _z) (Math|Vector|BreakVector _returnvalue))
  (return (* (Math|Vector|MakeVector (Math|Conversions|ToFloat(Integer) (Math|Float|Ceil _x)) (Math|Conversions|ToFloat(Integer) (Math|Float|Ceil _y)) (Math|Conversions|ToFloat(Integer) (Math|Float|Ceil _z))) _voxelsize)))

(fn Voxelization
  (for _array_element (Variables|Default|GetSampleDirectionList)
    (Variables|Default|SetSampleDirection _array_element)
    (CallFunction|1SetView)
    (CallFunction|2Sample)
    (CallFunction|3BuildInstanceMesh)))