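; Base zombie enemy character that provides attack, cry, patrol route and movement speed functions.
; Attack and Cry each play a montage on the mesh, then fire an end dispatcher whether it completes or is interrupted, so listeners always learn when the action finishes.
; SetMovementSpeed maps a movement-state enum to the walk speed, and a getter exposes the assigned patrol route.
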(event Custom|Cry
  (Animation|Montage|PlayMontage (Variables|Character|GetMesh) "/Game/ZombieCharacter/Montage/zombie_cry_Anim_Montage.zombie_cry_Anim_Montage"
    (:OnCompleted
      _)
    (:OnInterrupted
      _))
  (Default|CallOnCryEnd))

(event Custom|Attack
  (Animation|Montage|PlayMontage (Variables|Character|GetMesh) "/Game/ZombieCharacter/Montage/zombie_attack_Anim_Montage.zombie_attack_Anim_Montage"
    (:OnCompleted
      _)
    (:OnInterrupted
      _))
  (Default|CallOnAttackEnd))

(event EventBeginPlay)

(fn ConstructionScript)

(fn GetPartroRoute
  (return (Variables|AI|GetPartolRoute)))

(fn SetMovementSpeed
  (params (Speed :type E_MovementSpeed%20Enum :default "NewEnumerator0"))
  (Variables|/Script/Engine.CharacterMovementComponent|SetMaxWalkSpeed (Variables|Character|GetCharacterMovement) (Utilities|Select :Index Speed :NewEnumerator0 0.0 :NewEnumerator1 1e+02 :NewEnumerator2 3e+02 :NewEnumerator3 5e+02))
  (return 0.0))